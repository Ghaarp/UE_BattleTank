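; Player tank pawn Blueprint that handles camera aiming and firing, built from barrel, turret and two track meshes assigned in the construction script.
; On BeginPlay it passes barrel and turret to the TankAim component, passes both tracks to TankMovement, and zeroes the throttles.
; Aim axes yaw the azimuth gimbal and pitch the spring arm within a clamped range, while Fire calls TankAim.
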(event EventBeginPlay
  (Class|Tank|InitAimComponent (Variables|Default|GetTankAim) (Variables|Default|GetBarrel) (Variables|Default|GetTurret))
  (Class|Tank|InitMovementComponent (Variables|Default|GetTankMovement) (Variables|Default|GetLeftTrackTrue) (Variables|Default|GetRightTrackTrue))
  (Variables|Default|SetLeftThrottle 0.0)
  (Variables|Default|SetRightThrottle 0.0))

(event Input|ActionEvents|InputActionFire
  (params (Key :type Key%20Structure :default "None"))
  ;[1 1 1] CameraInput + Firing
  (:Pressed
    (Class|TankAimComponent|Fire (Variables|Default|GetTankAim))))

(event Input|AxisEvents|InputAxisAimAzimuth
  (params (AxisValue :type Float%20%28single-precision%29))
  ;[1 1 1] CameraInput + Firing
  (Transformation|AddLocalRotation (Variables|Default|GetAzimuthGimble) (Math|Rotator|MakeRotator 0.0 0.0 AxisValue) false false))

(event Input|AxisEvents|InputAxisAimAltitude
  (params (AxisValue :type Float%20%28single-precision%29))
  (bind _springarm (Variables|Default|GetSpringArm))
  (bind _returnvalue (Class|SpringArmComponent|GetTargetRotation _springarm))
  (bind _returnvalue_2 (+ AxisValue (.pitch _returnvalue)))
  ;[1 1 1] CameraInput + Firing
  (if (and (<= _returnvalue_2 1e+01) (<= -35.0 _returnvalue_2))
    (Transformation|AddLocalRotation (Variables|Default|GetSpringArm) (Math|Rotator|MakeRotator 0.0 AxisValue 0.0) false false)))

(fn ConstructionScript
  (Components|StaticMesh|SetStaticMesh (Variables|Default|GetBarrel) "/Game/Models/Tank/tank_fbx_Barrel.tank_fbx_Barrel")
  (Components|StaticMesh|SetStaticMesh (Variables|Default|GetTurret) "/Game/Models/Tank/tank_fbx_Turret.tank_fbx_Turret")
  (Components|StaticMesh|SetStaticMesh (Variables|Default|GetLeftTrackTrue) "/Game/Models/Tank/tank_fbx_Track.tank_fbx_Track")
  (Components|StaticMesh|SetStaticMesh (Variables|Default|GetRightTrackTrue) "/Game/Models/Tank/tank_fbx_Track.tank_fbx_Track"))